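; BP_LevelRestartTrigger is a trigger volume that restarts the current level when the player pawn enters it.
; On box overlap by player 0's pawn, it fades the camera to black and holds it, waits for the same FadeDelay, then reopens the current level by name.
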(event `self.BoxTrigger.OnComponentBeginOverlap`
  (params (OverlappedComponent :type "PrimitiveComponent Object Reference") (OtherActor :type "Actor Object Reference") (OtherComp :type "PrimitiveComponent Object Reference") (OtherBodyIndex :type Integer) (bFromSweep :type Boolean) (SweepResult :type "HitResult Structure (by ref)"))
  (if (== OtherActor (`GameplayStatics.GetPlayerPawn` 0))
    (`PlayerCameraManager.StartCameraFade` (`GameplayStatics.GetPlayerCameraManager` 0) 0.0 1.0 (`self.FadeDelay`) (struct :`A` 1.0) false true)
    (`KismetSystemLibrary.Delay` (`self.FadeDelay`))
    (bind _returnvalue (`GameplayStatics.GetCurrentLevelName` true))
    (`GameplayStatics.OpenLevel` (`KismetStringLibrary.Conv_StringToName` _returnvalue))))

(fn `UserConstructionScript`)