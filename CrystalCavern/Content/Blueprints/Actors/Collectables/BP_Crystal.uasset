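; BP_Crystal is a collectable actor that flies into the player's pawn and disappears on overlap.
; On overlap with player 0's pawn, it stores its location and plays a timeline whose alpha lerps it toward the pawn's current location each update, so it homes on a moving player.
; When the timeline finishes, the crystal destroys itself; no score or pickup effect is granted here.
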(event `self.ReceiveActorBeginOverlap`
  (params (OtherActor :type "Actor Object Reference"))
  (if (== OtherActor (`GameplayStatics.GetPlayerPawn` 0))
    (`self.StoreStartingValue`)
    (bind (_direction _smooth_lerp_alpha) (`Timeline|Alpha Blend TImeline`)
      (:`Update`
        (`self.MoveToPlayer` _smooth_lerp_alpha))
      (:`Finished`
        (`self.K2_DestroyActor`)))))

(fn `MoveToPlayer`
  (params (Alpha :type "Float (double-precision)"))
  (`self.K2_SetActorLocation` (`KismetMathLibrary.VLerp` (`self.LerpStartLocation`) (`self.K2_GetActorLocation` (`GameplayStatics.GetPlayerPawn` 0)) Alpha)))

(fn `StoreStartingValue`
  (set `self.LerpStartLocation` (`self.K2_GetActorLocation`)))

(fn `UserConstructionScript`)