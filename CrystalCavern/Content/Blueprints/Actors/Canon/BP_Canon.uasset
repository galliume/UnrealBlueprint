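; BP_Canon is a cannon actor that fires projectiles automatically and repeatedly from BeginPlay.
; Each cycle waits FireRate seconds, then spawns a BP_Projectile at ProjectileSpawnPoint's world location and rotation, scaled by ProjectileScale.
; CannonTimeline then animates the barrel along its relative Y axis, and its Cannon Fired event track loops execution back to the delay, so no separate timer is used.
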(event `self.ReceiveBeginPlay`
  (bind _projectilespawnpoint (`self.ProjectileSpawnPoint`))
  (`KismetSystemLibrary.Delay` (`self.FireRate`) :!label _label)
  (`|SpawnActorFromClass` "/Game/Blueprints/Actors/Projectiles/BP_Projectile.BP_Projectile_C" (`KismetMathLibrary.MakeTransform` (`SceneComponent.K2_GetComponentLocation` _projectilespawnpoint) (`SceneComponent.K2_GetComponentRotation` _projectilespawnpoint) (`KismetMathLibrary.Conv_DoubleToVector` (`self.ProjectileScale`))) "Undefined" "OverrideRootScale" null null)
  (bind (_direction _cannonbarrellocation) (`Timeline|CannonTimeline` :!via `PlayFromStart`)
    (:`Update`
      (`SceneComponent.K2_SetRelativeLocation` (`self.CannonBarrel`) (`KismetMathLibrary.MakeVector` 0.0 _cannonbarrellocation) false false))
    (:`CannonFired`
      (goto _label))))

(fn `UserConstructionScript`)